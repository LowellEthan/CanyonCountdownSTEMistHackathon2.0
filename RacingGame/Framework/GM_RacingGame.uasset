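; Game mode for a timed checkpoint race: after a start countdown, a timer runs until the player wins or runs out of time.
; On BeginPlay it binds to every BP_CheckPoint, separating the finish line from time-bonus checkpoints.
; Bonuses restart the timer with remaining plus added time and animate the HUD.
; Win or loss shows its screen, disables input, brakes the car and plays Level Sequences tagged Win or Lose.
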(event `self.ReceiveBeginPlay`
  ;[1 1 1] Rules_15:58
  (`|ExecutionSequence`
    (:`then_0`
      (bind _outactors (`GameplayStatics.GetAllActorsOfClass` "/Game/RacingGame/CheckPoint/BP_CheckPoint.BP_CheckPoint_C"))
      (for _array_element _outactors
        (bind _output_get (set `self.Is Finish Line_0` (`/Game/RacingGame/CheckPoint/BP_CheckPoint.isFinishLine` _array_element)))
        (if _output_get
          (add `/Game/RacingGame/CheckPoint/BP_CheckPoint.OneCHeckpointCrossed` _array_element (`|CreateDelegate` :!event `Win_CrossTheFinishLine`))
          (else
            (add `/Game/RacingGame/CheckPoint/BP_CheckPoint.OneCheckpointCrossedWIthTIme` _array_element (`|CreateDelegate` :!event `CrossedACheckpoint`))))))
    (:`then_1`
      (`self.StartCountdown`)
      (`self.PreRace`))))

(event `PreRace`
  (bind _returnvalue (`GameplayStatics.GetPlayerController` 0))
  (set `PlayerController.bShowMouseCursor` false _returnvalue)
  (`WidgetBlueprintLibrary.SetInputMode_GameOnly` _returnvalue))

(event `StartCountdown`
  ;[1 1 1] Rules_15:58
  (`KismetSystemLibrary.PrintString` "StartCountdown")
  (`KismetSystemLibrary.Delay` (`self.StartCountDownDuration`))
  (`self.GameStart`))

(event `Lose_OutOfTime`
  (bind _returnvalue (`GameplayStatics.GetPlayerController` 0))
  (bind _returnvalue_2 (`|CreateWidget` "/Game/RacingGame/UI/UserWidgetLoseScreen.UserWidgetLoseScreen_C"))
  (`UserWidget.AddToViewport` _returnvalue_2 0)
  (set `PlayerController.bShowMouseCursor` true _returnvalue)
  (`WidgetBlueprintLibrary.SetInputMode_GameAndUIEx` _returnvalue (`/Game/RacingGame/UI/UserWidgetLoseScreen.Button_0` _returnvalue_2))
  ;[1 1 1] Rules_15:58
  (`self.GameEnd` false))

(event `GameStart`
  ;[1 1 1] Rules_15:58
  (`KismetSystemLibrary.PrintString` "GameStart")
  (bind _returnvalue (`KismetSystemLibrary.K2_SetTimerDelegate` (delegate `Lose_OutOfTime`) (`self.GameStartTime`)))
  (set `self.TimeRemainingTime` _returnvalue))

(event `Win_CrossTheFinishLine`
  (bind _returnvalue (`GameplayStatics.GetPlayerController` 0))
  ;[1 1 1] Rules_15:58
  (`KismetSystemLibrary.K2_ClearAndInvalidateTimerHandle` (`self.TimeRemainingTime`))
  (bind _returnvalue_2 (`|CreateWidget` "/Game/RacingGame/UI/UserWidgetWinScreen.UserWidgetWinScreen_C"))
  (`UserWidget.AddToViewport` _returnvalue_2 0)
  (set `PlayerController.bShowMouseCursor` true _returnvalue)
  (`WidgetBlueprintLibrary.SetInputMode_GameAndUIEx` _returnvalue (`/Game/RacingGame/UI/UserWidgetWinScreen.Button_0` _returnvalue_2))
  (`self.GameEnd` true))

(event `GameEnd`
  (params (Win :type Boolean))
  (bind _returnvalue (`GameplayStatics.GetPlayerPawn` 0))
  ;[1 1 1] Rules_15:58
  (`KismetSystemLibrary.PrintString` (`KismetMathLibrary.SelectString` "You Win" "You Lose" Win))
  (`|ExecutionSequence`
    (:`then_0`
      (`self.DisableInput` _returnvalue (`GameplayStatics.GetPlayerController` 0))
      (bind _aswheeled_vehicle_pawn (cast `WheeledVehiclePawn` _returnvalue))
      (bind _vehiclemovementcomponent (`WheeledVehiclePawn.VehicleMovementComponent` _aswheeled_vehicle_pawn))
      (`ChaosVehicleMovementComponent.SetThrottleInput` _vehiclemovementcomponent 0.0)
      (`ChaosVehicleMovementComponent.SetHandbrakeInput` _vehiclemovementcomponent true)
      (`ChaosVehicleMovementComponent.SetSteeringInput` _vehiclemovementcomponent 1.0)
      (bind _asoffroad_car_pawn (cast `/Game/VehicleTemplate/Blueprints/OffroadCar/OffroadCar_Pawn` (`GameplayStatics.GetPlayerPawn` 0)))
      (`AudioComponent.Stop` (`/Game/VehicleTemplate/Blueprints/OffroadCar/OffroadCar_Pawn.SFX_Car_Engine` _asoffroad_car_pawn)))
    (:`then_1`
      (bind _outactors (`GameplayStatics.GetAllActorsOfClass` "/Script/LevelSequence.LevelSequenceActor"))
      (for _array_element _outactors
        (if (>= (`KismetArrayLibrary.Array_Find` (`Actor.Tags` _array_element) (select `bool` Win :`false` "Lose" :`true` "Win")) 0)
          (`MovieSceneSequencePlayer.Play` (`LevelSequenceActor.SequencePlayer` _array_element)))))))

(event `CrossedACheckpoint`
  (params (TimeToADD :type Integer))
  (`self.AddTimeToTimer` TimeToADD))

(fn `AddTimeToTimer`
  (params (TimeToAdd :type Integer))
  (bind _returnvalue (`KismetSystemLibrary.K2_SetTimerDelegate` (`|CreateDelegate` :!event `Lose_OutOfTime`) (+ (`KismetSystemLibrary.K2_GetTimerRemainingTimeHandle` (`self.TimeRemainingTime`)) (`local.TimeToAdd`))))
  (set `self.TimeRemainingTime` _returnvalue)
  (bind _asvehicle_player_controller (cast `/Game/VehicleTemplate/Blueprints/VehiclePlayerController` (`GameplayStatics.GetPlayerController` 0)))
  (`/Game/VehicleTemplate/Blueprints/VehicleUI.PlayAddedTImeAnim` (`/Game/VehicleTemplate/Blueprints/VehiclePlayerController.VehicleHud` _asvehicle_player_controller)))

(fn `NewFunction`)

(fn `UserConstructionScript`)